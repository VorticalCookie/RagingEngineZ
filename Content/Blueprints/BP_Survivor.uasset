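; On-foot survivor player character that moves by Enhanced Input while snapping to face the nearest zombie every tick and firing automatically.
; Game instance weapon type sets fire and magazine stats; a delay loop spawns projectiles, fanned for the shotgun, and auto-reloads from shared ammo.
; Overlaps message pickups through an interface; three Fix Car power-ups open the endless runner level.
; Death copies run stats to the game instance and shows the end screen.
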(event OnComponentBeginOverlap(CapsuleComponent)
  (params (OverlappedComponent :type Primitive%20Component%20Object%20Reference) (OtherActor :type Actor%20Object%20Reference) (OtherComp :type Primitive%20Component%20Object%20Reference) (OtherBodyIndex :type Integer) (bFromSweep :type Boolean) (SweepResult :type Hit%20Result%20Structure%20%28by%20ref%29))
  ;[0.15 0.15 0.15 0.5] PowerUp System
  (if (Utilities|DoesObjectImplementInterface OtherActor "/Game/Blueprints/DataStructures/BPI_SurvivorPickupable.BPI_SurvivorPickupable_C")
    (Class|BPISurvivorPickupable|OnSurvivorPickup(Message) OtherActor self)
    (Development|PrintString "PowerUp!")))

(event Death(AC_JohnHealth)
  (bind _game_instance (Variables|Default|GetGame%20Instance))
  ;[0.15 0.15 0.15 0.5] Swaps to Endscreen on Death
  (Variables|/Game/Blueprints/GameMode/BP_GameInstance.BP_GameInstance_C|SetFinalScore _game_instance (Variables|/Game/Blueprints/GameMode/BP_GameInstance.BP_GameInstance_C|GetScore _game_instance))
  (Variables|/Game/Blueprints/GameMode/BP_GameInstance.BP_GameInstance_C|SetFinalRunMoney _game_instance (Variables|/Game/Blueprints/GameMode/BP_GameInstance.BP_GameInstance_C|GetRunMoney _game_instance))
  (Variables|/Game/Blueprints/GameMode/BP_GameInstance.BP_GameInstance_C|SetFinalZombieKills _game_instance (Variables|/Game/Blueprints/GameMode/BP_GameInstance.BP_GameInstance_C|GetZombie%20Kills _game_instance))
  (Default|ChangetoEndScreen (Variables|Default|GetGame%20Instance)))

(event Custom|Shoot
  (bind _returnvalue (Transformation|GetActorTransform))
  ;[0.15 0.15 0.15 0.5] Spawn projectiles
  (Utilities|DelayLoop (Variables|Default|GetShotDelay) (not (Variables|Default|GetIsReloading?))
    (:Loop%20Body
      (Utilities|FlowControl|Delay (Variables|Default|GetShotDelay))
      (if (Variables|Default|GetShotgun?)
        (CallFunction|ShotgunSpread)
        (Math|Integer|DecrementInt (Variables|Default|GetAmmoInGun)
          (:%20%20
            (CallFunction|AmmoCheck)))
        (else
          (Game|SpawnActorfromClass "/Game/Blueprints/BP_Projectile.BP_Projectile_C" (Math|Transform|MakeTransform (+ (Math|Vector|RotateVector (Math|Vector|MakeVector (Variables|Default|GetProjectile%20Offset) 0.0 0.0) (.rotation _returnvalue)) (.location _returnvalue)) (.rotation _returnvalue) (.scale _returnvalue)) "Undefined" "MultiplyWithRoot" 0 0)
          (Math|Integer|DecrementInt (Variables|Default|GetAmmoInGun)
            (:%20%20
              (CallFunction|AmmoCheck))))))))

(event Custom|ActivatePowerUpType
  (params (NewPowerUpType :type SurvivorPowerUpTypes%20Enum :default "NewEnumerator0"))
  ;[0.15 0.15 0.15 0.5] PowerUp System
  (switch Utilities|FlowControl|Switch|SwitchonSurvivorPowerUpTypes NewPowerUpType
    (:NewEnumerator1
      (bind _result (Math|Integer|IncrementInt (Variables|Default|GetNeed%20to%20Fix))
        (:%20%20
          (if (>= _result 3)
            (Game|OpenLevel(byObjectReference) "/Game/Levels/LV_EndlessRuner.LV_EndlessRuner")))))))

(event Custom|Reload
  (bind _game_instance (Variables|Default|GetGame%20Instance))
  ;[0.15 0.15 0.15 0.5] Reloading
  (if (not (<= (Variables|/Game/Blueprints/GameMode/BP_GameInstance.BP_GameInstance_C|GetCurrentAmmo (Variables|Default|GetGame%20Instance)) 0))
    (Development|PrintString "Reloading..." true true "(R=1.000000,G=0.063994,B=0.000000,A=1.000000)" 4.0)
    (Utilities|FlowControl|Delay (Variables|Default|GetReloadSpeed))
    (Variables|Default|SetAmmoInGun (Math|Integer|Clamp(Integer) (Variables|/Game/Blueprints/GameMode/BP_GameInstance.BP_GameInstance_C|GetCurrentAmmo (Variables|Default|GetGame%20Instance)) 1 (Variables|Default|GetMagazineSize)))
    (Variables|/Game/Blueprints/GameMode/BP_GameInstance.BP_GameInstance_C|SetCurrentAmmo _game_instance (Math|Integer|Clamp(Integer) (- (Variables|/Game/Blueprints/GameMode/BP_GameInstance.BP_GameInstance_C|GetCurrentAmmo _game_instance) (Variables|Default|GetMagazineSize)) 0 (Variables|/Game/Blueprints/GameMode/BP_GameInstance.BP_GameInstance_C|GetCurrentAmmo _game_instance)))
    (Variables|Default|SetIsReloading? false)
    (CallFunction|Shoot)
    (else
      (Development|PrintString "RanOutOfAmmo" true true "(R=1.000000,G=0.000000,B=0.092591,A=1.000000)" 4.0))))

(event Custom|AmmoCheck
  ;[0.15 0.15 0.15 0.5] Reloading
  (if (<= (Variables|Default|GetAmmoInGun) 0)
    (Development|PrintString "Need to reload")
    (CallFunction|Reload)
    (Variables|Default|SetIsReloading? true)))

(event Custom|CheckWeapon
  ;[0.15 0.15 0.15 0.5] Check Weapon
  (switch Utilities|FlowControl|Switch|SwitchonWeaponTypes (Variables|/Game/Blueprints/GameMode/BP_GameInstance.BP_GameInstance_C|GetWeaponTypes (Variables|Default|GetGame%20Instance))
    (:NewEnumerator0
      (Variables|Default|SetShotDelay 0.5)
      (Variables|Default|SetMagazineSize 16)
      (Variables|Default|SetAmmoInGun 16)
      (Variables|Default|SetReloadSpeed 1.25))
    (:NewEnumerator1
      (Variables|Default|SetShotDelay 0.3)
      (Variables|Default|SetMagazineSize 36)
      (Variables|Default|SetAmmoInGun 36)
      (Variables|Default|SetReloadSpeed 2.0))
    (:NewEnumerator2
      (Variables|Default|SetShotDelay 1.25)
      (Variables|Default|SetMagazineSize 6)
      (Variables|Default|SetAmmoInGun 6)
      (Variables|Default|SetReloadSpeed 3.0)
      (Variables|Default|SetShotgun? true))))

(event Custom|Shotgun%20Spread
  (bind _returnvalue (Transformation|GetActorTransform))
  ;[0.15 0.15 0.15 0.5] Shotgun Spread
  (for _index (range 1 (Variables|Default|GetShotgun%20Projectile%20Amount))
    (Game|SpawnActorfromClass "/Game/Blueprints/BP_Projectile.BP_Projectile_C" (Math|Transform|MakeTransform (+ (Math|Vector|RotateVector (Math|Vector|MakeVector (Variables|Default|GetProjectile%20Offset) 0.0 0.0) (.rotation _returnvalue)) (.location _returnvalue)) (Math|Rotator|CombineRotators (.rotation _returnvalue) (* (Math|Rotator|MakeRotator 0.0 0.0 (Variables|Default|GetSpread)) _index)) (.scale _returnvalue)) "Undefined" "MultiplyWithRoot" 0 0)))

(event Input|EnhancedActionEvents|EnhancedInputActionIA_SMove
  (params (ActionValue :type Vector%202D%20Structure) (ElapsedSeconds :type Float%20%28double-precision%29) (TriggeredSeconds :type Float%20%28double-precision%29) (InputAction :type Input%20Action%20Object%20Reference :default "/Game/Inputs/Survivor/IA_SMove.IA_SMove"))
  ;[0.15 0.15 0.15 0.5] Movement
  (Variables|Default|SetLast%20Move (Math|Vector2D|MakeVector2D (.x ActionValue) (.y ActionValue)))
  (CallFunction|Move (.x ActionValue) (.y ActionValue)))

(event EventBeginPlay
  (bind _returnvalue (Game|GetGameInstance))
  ;[0.15 0.15 0.15 0.5] Movement
  (bind _returnvalue_2 (UserInterface|CreateWidget "/Game/UI/UI_On_Foot.UI_On_Foot_C" (Game|GetPlayerController 0)))
  (UserInterface|Viewport|AddtoViewport _returnvalue_2 0)
  (Utilities|FlowControl|Sequence
    (:then_0
      (Input|AddMappingContext (PlayerController|LocalPlayerSubsystems|GetEnhancedInputLocalPlayerSubsystem (Game|GetPlayerController 0)) "/Game/Inputs/Survivor/IMC_Survivor.IMC_Survivor" 0 "(bIgnoreAllPressedKeysUntilRelease=True,bForceImmediately=False,bNotifyUserSettings=False)"))
    (:then_1
      (Utilities|IsValid _returnvalue
        (:Is%20Valid
          (bind _asbp_game_instance (Utilities|Casting|CastToBP_GameInstance _returnvalue))
          (Variables|Default|SetGame%20Instance _asbp_game_instance)
          (CallFunction|CheckWeapon))))
    (:then_2
      (CallFunction|Shoot))))

(event EventTick
  (params (DeltaSeconds :type Float%20%28single-precision%29))
  (bind _returnvalue (Transformation|GetActorLocation))
  ;[0.15 0.15 0.15 0.5] Old camera movement
  (bind _outactors (Actor|GetAllActorsOfClass "/Game/Blueprints/Zombies/BP_Zombie.BP_Zombie_C"))
  (Variables|Default|SetTargetRotation (.yaw (Math|Rotator|FindLookatRotation _returnvalue (Transformation|GetActorLocation (.ReturnValue (Actor|FindNearestActor _returnvalue _outactors))))))
  (CallFunction|SnapPlayer))

(event Input|KeyboardEvents|1
  (params (Key :type Key%20Structure :default "None"))
  ;[0.15 0.15 0.15 0.5] Press 1 key to deal damage to John
  (:Pressed
    (Default|TakeDamage (Variables|Default|GetAC_JohnHealth) 1)))

(fn ConstructionScript)

(fn Move
  (params (Axis%20X :type Float%20%28double-precision%29) (Axis%20Y :type Float%20%28double-precision%29))
  (bind _returnvalue (Pawn|GetControlRotation :!class /Script/Engine.Pawn))
  (bind _returnvalue_2 (Pawn|GetControlRotation :!class /Script/Engine.Pawn))
  (Pawn|Input|AddMovementInput (Math|Vector|GetForwardVector (Math|Rotator|MakeRotator (.roll _returnvalue_2) 0.0 (.yaw _returnvalue_2))) Axis%20X false)
  (Pawn|Input|AddMovementInput (Math|Vector|GetRightVector (Math|Rotator|MakeRotator (.roll _returnvalue) 0.0 (.yaw _returnvalue))) Axis%20Y false))

(fn RotatePlayer
  (bind _returnvalue (Transformation|GetActorRotation))
  (if (not (Math|Float|NearlyEqual(Float) (.yaw _returnvalue) (Variables|Default|GetTargetRotation) 0.5))
    (Transformation|SetActorRotation (Math|Rotator|MakeRotator (.roll _returnvalue) (.pitch _returnvalue) (.yaw (Math|Interpolation|RInterpTo (Transformation|GetActorRotation) (Math|Rotator|MakeRotator (.roll _returnvalue) (.pitch _returnvalue) (Variables|Default|GetTargetRotation)) (Utilities|Time|GetWorldDeltaSeconds) 1e+01))))
    (return)))

(fn SnapPlayer
  (bind _returnvalue (Transformation|GetActorRotation))
  (Transformation|SetActorRotation (Math|Rotator|MakeRotator (.roll _returnvalue) (.pitch _returnvalue) (Variables|Default|GetTargetRotation)))
  (return))
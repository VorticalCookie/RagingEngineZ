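; Extraction zone actor where the survivor holds position to extract, hidden and non-colliding on reset and revealed with ready and engine sounds on activation.
; Survivor overlap starts a hold timer and a timeline that drives the on-foot UI progress through the Game Instance.
; Leaving cancels both and hides the UI.
; Finishing stores the player's health in the Game Instance and calls its Extraction.
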(event OnComponentBeginOverlap(ExtractionCollision)
  (params (OverlappedComponent :type Primitive%20Component%20Object%20Reference) (OtherActor :type Actor%20Object%20Reference) (OtherComp :type Primitive%20Component%20Object%20Reference) (OtherBodyIndex :type Integer) (bFromSweep :type Boolean) (SweepResult :type Hit%20Result%20Structure%20%28by%20ref%29))
  (Utilities|Casting|CastToBP_Survivor OtherActor)
  (if (not (Variables|Default|GetbExtractionInProgress))
    (Variables|Default|SetbIsPlayerinZone true)
    (Variables|Default|SetbExtractionInProgress true)
    (bind _asbp_game_instance (Utilities|Casting|CastToBP_GameInstance (Game|GetGameInstance)))
    (Utilities|IsValid (Variables|/Game/Blueprints/GameMode/BP_GameInstance.BP_GameInstance_C|GetUIonFootRef _asbp_game_instance)
      (:Is%20Valid
        (Default|ShowExtractionUI (Variables|/Game/Blueprints/GameMode/BP_GameInstance.BP_GameInstance_C|GetUIonFootRef _asbp_game_instance))
        (bind _returnvalue (Utilities|Time|SetTimerbyEvent (delegate Custom|FinishExtraction) (Variables|Default|GetExtractionHoldTime)))
        (Variables|Default|SetExtractTimerHandle _returnvalue)
        (bind _extraction (Timeline|ExtractionProgress PlayFromStart)
          (:Update
            (bind _asbp_game_instance_2 (Utilities|Casting|CastToBP_GameInstance (Game|GetGameInstance)))
            (Utilities|IsValid (Variables|/Game/Blueprints/GameMode/BP_GameInstance.BP_GameInstance_C|GetUIonFootRef _asbp_game_instance_2)
              (:Is%20Valid
                (Default|SetExtractionProgress (Variables|/Game/Blueprints/GameMode/BP_GameInstance.BP_GameInstance_C|GetUIonFootRef _asbp_game_instance_2) _extraction)))))))))

(event OnComponentEndOverlap(ExtractionCollision)
  (params (OverlappedComponent :type Primitive%20Component%20Object%20Reference) (OtherActor :type Actor%20Object%20Reference) (OtherComp :type Primitive%20Component%20Object%20Reference) (OtherBodyIndex :type Integer))
  (Utilities|Casting|CastToBP_Survivor OtherActor)
  (Variables|Default|SetbIsPlayerinZone false)
  (Variables|Default|SetbExtractionInProgress false)
  (Utilities|Time|ClearandInvalidateTimerbyHandle (Variables|Default|GetExtractTimerHandle))
  (Audio|Components|Audio|Stop (Variables|Default|GetExtractionProgress))
  (bind _asbp_game_instance (Utilities|Casting|CastToBP_GameInstance (Game|GetGameInstance)))
  (Utilities|IsValid (Variables|/Game/Blueprints/GameMode/BP_GameInstance.BP_GameInstance_C|GetUIonFootRef _asbp_game_instance)
    (:Is%20Valid
      (Default|HideExtractionUI (Variables|/Game/Blueprints/GameMode/BP_GameInstance.BP_GameInstance_C|GetUIonFootRef _asbp_game_instance)))))

(event Custom|ActivateExtractionZone
  ;[0.15 0.15 0.15 0.5] Activates the Extraction Zone/Sounds
  (Audio|PlaySound2D "/Game/SFX/Car_Sounds/Extraction_Ready.Extraction_Ready" 1.0 1.0 0.0 0 0)
  (Development|SetHiddeninGame (Variables|Default|GetZoneMesh) false false)
  (Collision|SetCollisionEnabled (Variables|Default|GetExtraction%20Collision) "QueryAndPhysics")
  (Utilities|FlowControl|Delay 1.5)
  (Audio|SpawnSoundatLocation "/Game/SFX/Car_Sounds/Engine_Drive.Engine_Drive" (Transformation|GetWorldLocation (Variables|Default|GetDefaultSceneRoot)) "0, 0, 0" 1.0 1.0 0.0 "/Game/SFX/Car_Sounds/SA_ExtractionReady.SA_ExtractionReady" 0))

(event Custom|FinishExtraction
  (if (Variables|Default|GetbIsPlayerinZone)
    (bind _asbp_game_instance (Utilities|Casting|CastToBP_GameInstance (Game|GetGameInstance)))
    (Utilities|IsValid (Variables|/Game/Blueprints/GameMode/BP_GameInstance.BP_GameInstance_C|GetUIonFootRef _asbp_game_instance)
      (:Is%20Valid
        (Default|SetExtractionProgress (Variables|/Game/Blueprints/GameMode/BP_GameInstance.BP_GameInstance_C|GetUIonFootRef _asbp_game_instance) 1.0)
        (Default|HideExtractionUI (Variables|/Game/Blueprints/GameMode/BP_GameInstance.BP_GameInstance_C|GetUIonFootRef _asbp_game_instance))
        (bind _asbp_survivor (Utilities|Casting|CastToBP_Survivor (Game|GetPlayerCharacter 0)))
        (Variables|/Game/Blueprints/GameMode/BP_GameInstance.BP_GameInstance_C|SetJohnHP (Variables|Default|GetGame%20Instance) (Variables|/Game/Blueprints/AC_JohnHealth.AC_JohnHealth_C|GetHealth (Variables|/Game/Blueprints/BP_Survivor.BP_Survivor_C|GetAC_JohnHealth _asbp_survivor)))
        (Variables|/Game/Blueprints/GameMode/BP_GameInstance.BP_GameInstance_C|SetJohnHPStored _asbp_game_instance true)
        (Default|Extraction _asbp_game_instance)))))

(event Custom|ResetExtractionZone
  ;[0.15 0.15 0.15 0.5] Function to Reset Extraction Booleans/State for exiting
  (Development|SetHiddeninGame (Variables|Default|GetZoneMesh) true false)
  (Collision|SetCollisionEnabled (Variables|Default|GetExtraction%20Collision) "NoCollision")
  (Variables|Default|SetbIsPlayerinZone false)
  (Variables|Default|SetbExtractionInProgress false)
  (Utilities|Time|ClearandInvalidateTimerbyHandle (Variables|Default|GetExtractTimerHandle))
  (Audio|Components|Audio|Stop (Variables|Default|GetExtractionProgress)))

(event EventBeginPlay
  ;[0.15 0.15 0.15 0.5] Gets Game Instance Ref
  (bind _asbp_game_instance (Utilities|Casting|CastToBP_GameInstance (Game|GetGameInstance)))
  (Variables|Default|SetGame%20Instance _asbp_game_instance))

(event EventTick
  (params (DeltaSeconds :type Float%20%28single-precision%29)))

(fn ConstructionScript)
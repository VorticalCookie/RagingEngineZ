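; Floor tile for a three-lane endless game that moves itself along negative X every tick at a fixed speed.
; SpawnObstacle and SpawnPowerUp attach the given class as a child actor at the left, middle or right lane start point.
; When BP_TestPawn overlaps DestroyTileCollision, the tile messages the game mode to add a new tile, removes itself from ActiveTiles and destroys itself.
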(event OnComponentBeginOverlap(DestroyTileCollision)
  (params (OverlappedComponent :type Primitive%20Component%20Object%20Reference) (OtherActor :type Actor%20Object%20Reference) (OtherComp :type Primitive%20Component%20Object%20Reference) (OtherBodyIndex :type Integer) (bFromSweep :type Boolean) (SweepResult :type Hit%20Result%20Structure%20%28by%20ref%29))
  (Utilities|Casting|CastToBP_TestPawn OtherActor)
  (Development|PrintString "New Tile")
  (Class|BPINewTile|AddNewTile(Message) (Game|GetGameMode))
  (Utilities|Array|RemoveItem (Variables|/Game/Blueprints/GameMode/BP_EndlessGameMode.BP_EndlessGameMode_C|GetActiveTiles (Variables|Default|GetGameMode_Ref)) self)
  (Actor|DestroyActor))

(event Custom|SpawnPowerUp
  (params (PowerUp%20Class :type BP%20Power%20Up%20Class%20Reference) (Lane%20Number :type Integer))
  ;[0.15 0.15 0.15 0.5] Spawn PowerUp
  (bind _returnvalue (AddComponent|AddChildActorComponent false (Math|Transform|MakeTransform (Variables|/Script/Engine.SceneComponent|GetRelativeLocation (Utilities|Select :Index Lane%20Number :Option%200 (Variables|Default|GetStartPointL) :Option%201 (Variables|Default|GetStartPointM) :Option%202 (Variables|Default|GetStartPointR))) "0, 0, 0" "1.000000,1.000000,1.000000")))
  (ChildActorComponent|SetChildActorClass _returnvalue PowerUp%20Class))

(event Custom|SpawnObstacle
  (params (Obstacle%20Class :type BP%20Obstacle%20Class%20Reference) (Lane%20Number :type Integer))
  ;[0.15 0.15 0.15 0.5] Spawn Obstacle
  (bind _returnvalue (AddComponent|AddChildActorComponent false (Math|Transform|MakeTransform (Variables|/Script/Engine.SceneComponent|GetRelativeLocation (Utilities|Select :Index Lane%20Number :Option%200 (Variables|Default|GetStartPointL) :Option%201 (Variables|Default|GetStartPointM) :Option%202 (Variables|Default|GetStartPointR))) "0, 0, 0" "1.000000,1.000000,1.000000")))
  (ChildActorComponent|SetChildActorClass _returnvalue Obstacle%20Class))

(event EventTick
  (params (DeltaSeconds :type Float%20%28single-precision%29))
  (Transformation|AddActorWorldOffset (* (Utilities|Time|GetWorldDeltaSeconds) "-500.000000,0.000000,0.000000")))

(event EventBeginPlay
  (bind _asbp_endless_game_mode (Utilities|Casting|CastToBP_EndlessGameMode (Game|GetGameMode)))
  (Variables|Default|SetGameMode_Ref _asbp_endless_game_mode))

(fn ConstructionScript)
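; BP_FireTrail is a fire trail actor that follows the player's survivor and damages zombies it touches.
; On BeginPlay it targets the BP_Survivor player pawn.
; Each tick, while at or beyond the follow distance, it moves toward the target at constant speed, keeping its height and yawing to face it.
; Overlaps on the FireTrail component deal damage without knockback through AC_ZombieHealth.
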(event OnComponentBeginOverlap(FireTrail)
  (params (OverlappedComponent :type Primitive%20Component%20Object%20Reference) (OtherActor :type Actor%20Object%20Reference) (OtherComp :type Primitive%20Component%20Object%20Reference) (OtherBodyIndex :type Integer) (bFromSweep :type Boolean) (SweepResult :type Hit%20Result%20Structure%20%28by%20ref%29))
  (bind _returnvalue (Actor|GetComponentbyClass OtherActor "/Game/Blueprints/AC_ZombieHealth.AC_ZombieHealth_C"))
  (Utilities|IsValid _returnvalue
    (:Is%20Valid
      (Default|TakeDamage _returnvalue (Variables|Default|GetDamage) false))))

(event EventTick
  (params (DeltaSeconds :type Float%20%28single-precision%29))
  (bind _returnvalue (Transformation|GetActorLocation))
  (bind _movespeed (Variables|Default|GetMoveSpeed))
  (bind _target (Variables|Default|GetTarget))
  (bind _returnvalue_2 (Transformation|GetActorLocation _target))
  (bind _returnvalue_3 (Math|Interpolation|VInterptoConstant _returnvalue _returnvalue_2 DeltaSeconds _movespeed))
  (bind (_x _y) (Math|Vector|BreakVector _returnvalue_3))
  (Utilities|IsValid _target
    (:Is%20Valid
      (if (>= (Math|Vector|Distance(Vector) _returnvalue _returnvalue_2) (Variables|Default|GetFollowDis))
        (Transformation|SetActorLocationAndRotation (Math|Vector|MakeVector _x _y (.z (Transformation|GetActorLocation))) (Math|Rotator|MakeRotator 0.0 0.0 (.yaw (Math|Rotator|FindLookatRotation _returnvalue_3 _returnvalue_2))))))
    (:Is%20Not%20Valid
      (Development|PrintString "No Target Set"))))

(event EventBeginPlay
  (bind _asbp_survivor (Utilities|Casting|CastToBP_Survivor (Game|Player|GetPlayerPawn 0)))
  (Variables|Default|SetTarget _asbp_survivor))

(fn ConstructionScript)
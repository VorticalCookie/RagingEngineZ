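; Crate power-up pickup that plays a sound and grants the survivor a random power when collected.
; RollCratePower picks between a full-health Medkit, an Ammo Cache, timed Instant Kill and timed Pay Day, applying them through BP_Survivor and BP_GameInstance.
; Timed powers recursively reroll when the game instance disallows activation.
; The actor destroys itself after granting, though Medkit and Ammo only do so if the on-foot UI is valid.
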(event EventBeginPlay
  (|CallParentFunction) ; This node is disabled and will not be called.\nDrag off pins to build functionality.
)

(event Collision|EventActorBeginOverlap
  (params (OtherActor :type Actor%20Object%20Reference))
  (|CallParentFunction OtherActor))

(event EventTick
  (params (DeltaSeconds :type Float%20%28single-precision%29)))

(event EventOnSurvivorPickup
  (params (InteractingPlayer :type BP%20Survivor%20Object%20Reference))
  (Audio|PlaySound2D "/Game/SFX/CratePowerUp.CratePowerUp" 1.0 1.0 0.0 0 0)
  (CallFunction|RollCratePower))

(fn ConstructionScript
  (|CallParentFunction))

(fn RollCratePower
  (switch Utilities|FlowControl|Switch|SwitchonE_CratePowerUps (Utilities|Enum|ByteToEnumE_CratePowerUps (Math|Conversions|ToByte(Integer) (Math|Random|RandomIntegerinRange 0 3)))
    (:NewEnumerator0
      ;[0.15 0.15 0.15 0.5] Medkit, heals John 100%
      (Development|PrintString "Medkit")
      (bind _asbp_survivor (Utilities|Casting|CastToBP_Survivor (Game|GetPlayerCharacter 0)))
      (Variables|/Game/Blueprints/AC_JohnHealth.AC_JohnHealth_C|SetHealth (Variables|/Game/Blueprints/BP_Survivor.BP_Survivor_C|GetAC_JohnHealth _asbp_survivor) (Variables|/Game/Blueprints/AC_JohnHealth.AC_JohnHealth_C|GetMax%20Health (Variables|/Game/Blueprints/BP_Survivor.BP_Survivor_C|GetAC_JohnHealth _asbp_survivor)))
      (bind _asbp_game_instance (Utilities|Casting|CastToBP_GameInstance (Game|GetGameInstance)))
      (Utilities|IsValid (Variables|/Game/Blueprints/GameMode/BP_GameInstance.BP_GameInstance_C|GetUIonFootRef _asbp_game_instance)
        (:Is%20Valid
          (Default|ShowMedkitText (Variables|/Game/Blueprints/GameMode/BP_GameInstance.BP_GameInstance_C|GetUIonFootRef _asbp_game_instance) "Applying Medkit")
          (Actor|DestroyActor))))
    (:NewEnumerator1
      ;[0.15 0.15 0.15 0.5] Ammo Cache, gives 100 ammo
      (Development|PrintString "Ammo Cache")
      (bind _asbp_game_instance_2 (Utilities|Casting|CastToBP_GameInstance (Game|GetGameInstance)))
      (Variables|/Game/Blueprints/GameMode/BP_GameInstance.BP_GameInstance_C|SetCurrentAmmo _asbp_game_instance_2 (+ (Variables|/Game/Blueprints/GameMode/BP_GameInstance.BP_GameInstance_C|GetCurrentAmmo _asbp_game_instance_2) (Variables|Default|GetAmmo%20to%20add)))
      (Utilities|IsValid (Variables|/Game/Blueprints/GameMode/BP_GameInstance.BP_GameInstance_C|GetUIonFootRef _asbp_game_instance_2)
        (:Is%20Valid
          (Default|ShowAmmoText (Variables|/Game/Blueprints/GameMode/BP_GameInstance.BP_GameInstance_C|GetUIonFootRef _asbp_game_instance_2) "Obtained Ammo Cache")
          (Actor|DestroyActor))))
    (:NewEnumerator2
      ;[0.15 0.15 0.15 0.5] Instant Kill, kill all zombies in one shot
      (Development|PrintString "Instant Kill")
      (bind _asbp_game_instance_3 (Utilities|Casting|CastToBP_GameInstance (Game|GetGameInstance)))
      (bind _canactivate (Default|CanActivateTimedPower _asbp_game_instance_3))
      (if _canactivate
        (Default|StartTimedPower _asbp_game_instance_3 "NewEnumerator2" 15.0)
        (bind _asbp_survivor_2 (Utilities|Casting|CastToBP_Survivor (Game|GetPlayerCharacter 0)))
        (Default|ActivateInstantKill _asbp_survivor_2 15.0)
        (Actor|DestroyActor)
        (else
          (CallFunction|RollCratePower))))
    (:NewEnumerator3
      ;[0.15 0.15 0.15 0.5] Pay Day, double money gain
      (Development|PrintString "Pay Day")
      (bind _asbp_game_instance_4 (Utilities|Casting|CastToBP_GameInstance (Game|GetGameInstance)))
      (bind _canactivate_2 (Default|CanActivateTimedPower _asbp_game_instance_4))
      (if _canactivate_2
        (Default|StartTimedPower _asbp_game_instance_4 "NewEnumerator3" 2e+01)
        (bind _asbp_game_instance_5 (Utilities|Casting|CastToBP_GameInstance (Game|GetGameInstance)))
        (Default|ActivatePayDay _asbp_game_instance_5 2e+01)
        (Actor|DestroyActor)
        (else
          (CallFunction|RollCratePower))))))
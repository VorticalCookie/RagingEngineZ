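; Repair parts power-up actor that restores a fifth of the car's maximum armor when picked up, then destroys itself.
; Both pickup events play a sound and call AddCarHealth, which raises the clamped CarArmor on BP_GameInstance and rechecks the extraction condition.
; An unconnected older chain that also copied armor into BP_Car's health component never runs, and debug prints remain.
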(event Custom|Add%20Car%20Health
  ;[0.15 0.15 0.15 0.5] Repair parts heals game instance variable
  (bind _asbp_game_instance (Utilities|Casting|CastToBP_GameInstance (Game|GetGameInstance)))
  (bind _output_get (Variables|/Game/Blueprints/GameMode/BP_GameInstance.BP_GameInstance_C|SetCar%20Armor _asbp_game_instance (Math|Integer|Clamp(Integer) (+ (Variables|/Game/Blueprints/GameMode/BP_GameInstance.BP_GameInstance_C|GetCar%20Armor _asbp_game_instance) (* (Math|Conversions|ToFloat(Integer) (Variables|/Game/Blueprints/GameMode/BP_GameInstance.BP_GameInstance_C|GetCar%20Armor%20Max _asbp_game_instance)) 0.2)) 1 (Variables|/Game/Blueprints/GameMode/BP_GameInstance.BP_GameInstance_C|GetCar%20Armor%20Max _asbp_game_instance))))
  (Default|CheckExtractionCondition (Variables|Default|GetGameInstance%20Ref))
  (Development|PrintString (Utilities|String|ToString(Integer) _output_get)))

(event EventBeginPlay)

(event Collision|EventActorBeginOverlap
  (params (OtherActor :type Actor%20Object%20Reference)))

(event EventTick
  (params (DeltaSeconds :type Float%20%28single-precision%29)))

(event EventOnPickedUp
  (params (Interacting%20Player :type BP%20Car%20Object%20Reference))
  (Development|PrintString "Picked up power")
  (Audio|PlaySound2D "/Game/SFX/Pickup_Resource_V2.Pickup_Resource_V2" 1.0 1.0 0.0 0 0)
  (CallFunction|AddCarHealth)
  (Actor|DestroyActor))

(event EventOnSurvivorPickup
  (params (InteractingPlayer :type BP%20Survivor%20Object%20Reference))
  (Development|PrintString "Picked up power")
  (Audio|PlaySound2D "/Game/SFX/Pickup_Resource_V2.Pickup_Resource_V2" 1.0 1.0 0.0 0 0)
  (CallFunction|AddCarHealth)
  (Actor|DestroyActor))

(fn ConstructionScript
  (|CallParentFunction))
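; BP_GasPickup is a gas power-up that refills the car's gas through the game instance, building on a parent pickup's overlap handling.
; OnPickedUp plays a sound, calls RepairGasPart on the game instance and destroys the actor.
; OnSurvivorPickup instead adds a tenth of max gas, clamped, then checks the extraction condition.
; That path updates the on-foot UI and destroys the actor only when that UI reference is valid.
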(event Custom|Add%20Car%20Gas
  (bind _asbp_game_instance (Utilities|Casting|CastToBP_GameInstance (Game|GetGameInstance)))
  (Variables|/Game/Blueprints/GameMode/BP_GameInstance.BP_GameInstance_C|SetCarCurrentGas _asbp_game_instance (Math|Float|Clamp(Float) (+ (Variables|/Game/Blueprints/GameMode/BP_GameInstance.BP_GameInstance_C|GetCarCurrentGas _asbp_game_instance) (* (Variables|/Game/Blueprints/GameMode/BP_GameInstance.BP_GameInstance_C|GetCarMaxGas _asbp_game_instance) 0.1)) 0.0 (Variables|/Game/Blueprints/GameMode/BP_GameInstance.BP_GameInstance_C|GetCarMaxGas _asbp_game_instance)))
  (Default|CheckExtractionCondition (Variables|Default|GetGameInstance%20Ref)))

(event EventTick
  (params (DeltaSeconds :type Float%20%28single-precision%29)))

(event EventOnPickedUp
  (params (Interacting%20Player :type BP%20Car%20Object%20Reference))
  (Development|PrintString "Picked up power")
  (Audio|PlaySound2D "/Game/SFX/Pickup_Resource_V2.Pickup_Resource_V2" 1.0 1.0 0.0 0 0)
  (Default|RepairGasPart (Variables|Default|GetGameInstance%20Ref))
  (Actor|DestroyActor))

(event EventOnSurvivorPickup
  (params (InteractingPlayer :type BP%20Survivor%20Object%20Reference))
  (Development|PrintString "Picked up power")
  (Audio|PlaySound2D "/Game/SFX/Pickup_Resource_V2.Pickup_Resource_V2" 1.0 1.0 0.0 0 0)
  (CallFunction|AddCarGas)
  (bind _asbp_game_instance (Utilities|Casting|CastToBP_GameInstance (Game|GetGameInstance)))
  (Utilities|IsValid (Variables|/Game/Blueprints/GameMode/BP_GameInstance.BP_GameInstance_C|GetUIonFootRef _asbp_game_instance)
    (:Is%20Valid
      (Default|UpdateCarGasUI (Variables|/Game/Blueprints/GameMode/BP_GameInstance.BP_GameInstance_C|GetUIonFootRef _asbp_game_instance))
      (Actor|DestroyActor))))

(event Collision|EventActorBeginOverlap
  (params (OtherActor :type Actor%20Object%20Reference))
  (|CallParentFunction OtherActor))

(fn ConstructionScript
  (|CallParentFunction))
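; BP_Ammo is an ammo power-up pickup that adds a fixed amount to the current ammo count stored on the game instance.
; It extends a parent pickup, calling the parent logic in both OnPickedUp and OnSurvivorPickup before adding the ammo.
; The survivor pickup path also activates a power-up type on the interacting player.
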(event EventBeginPlay)

(event Collision|EventActorBeginOverlap
  (params (OtherActor :type Actor%20Object%20Reference)))

(event EventTick
  (params (DeltaSeconds :type Float%20%28single-precision%29)))

(event EventOnPickedUp
  (params (Interacting%20Player :type BP%20Car%20Object%20Reference))
  (bind _gameinstance_ref (Variables|Default|GetGameInstance%20Ref))
  (|CallParentFunction Interacting%20Player)
  (Variables|/Game/Blueprints/GameMode/BP_GameInstance.BP_GameInstance_C|SetCurrentAmmo _gameinstance_ref (+ (Variables|/Game/Blueprints/GameMode/BP_GameInstance.BP_GameInstance_C|GetCurrentAmmo _gameinstance_ref) 6)))

(event EventOnSurvivorPickup
  (params (InteractingPlayer :type BP%20Survivor%20Object%20Reference))
  (bind _gameinstance_ref (Variables|Default|GetGameInstance%20Ref))
  (|CallParentFunction InteractingPlayer)
  (Variables|/Game/Blueprints/GameMode/BP_GameInstance.BP_GameInstance_C|SetCurrentAmmo _gameinstance_ref (+ (Variables|/Game/Blueprints/GameMode/BP_GameInstance.BP_GameInstance_C|GetCurrentAmmo _gameinstance_ref) 6))
  (Default|ActivatePowerUpType InteractingPlayer "NewEnumerator2"))

(fn ConstructionScript
  (|CallParentFunction))
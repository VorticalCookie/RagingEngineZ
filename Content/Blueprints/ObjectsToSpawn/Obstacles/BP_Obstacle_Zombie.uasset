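; Zombie obstacle that awards money and a kill on any actor overlap, then plays a random death sound and destroys itself a tick later.
; With the LV10CarGas upgrade, a kill can also grant extra gas by chance.
; On spawn it randomizes mesh yaw and sets the anim blueprint's AnimSpeed to either moving or zero.
; Tick derives InterpSpeed from mesh displacement, though this graph never reads it.
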(event EventBeginPlay
  (Class|AudioMixerBlueprintLibrary|PrimeSoundCueforPlayback "/Game/SFX/SC_Zombie_Death_Random.SC_Zombie_Death_Random")
  (|CallParentFunction)
  (Variables|Default|SetPreviousLocation (Transformation|GetWorldLocation (Variables|Default|GetSkeletalMesh)))
  (Transformation|SetRelativeRotation (Variables|Default|GetSkeletalMesh) (Math|Rotator|MakeRotator 0.0 0.0 (.yaw (Math|Rotator|MakeRotator 0.0 0.0 (Math|Random|RandomFloatinRange 0.0 3.6e+02)))) false false)
  (bind _asabp_zombie_obstacle (Utilities|Casting|CastToABP_ZombieObstacle (Components|SkeletalMesh|GetAnimInstance (Variables|Default|GetSkeletalMesh))))
  (if (Math|Random|RandomBool)
    (Variables|/Game/Models/Animations/Zombie/ABP_ZombieObstacle.ABP_ZombieObstacle_C|SetAnimSpeed _asabp_zombie_obstacle 3e+02)
    (else
      (Variables|/Game/Models/Animations/Zombie/ABP_ZombieObstacle.ABP_ZombieObstacle_C|SetAnimSpeed _asabp_zombie_obstacle 0.0))))

(event Collision|EventActorBeginOverlap
  (params (OtherActor :type Actor%20Object%20Reference))
  (bind _gameinstanceref (Variables|Default|GetGameInstanceRef))
  (|CallParentFunction OtherActor)
  (Default|AddMoney _gameinstanceref)
  (Default|AddZombieKills _gameinstanceref)
  (if (and (Variables|/Game/Blueprints/GameMode/BP_GameInstance.BP_GameInstance_C|GetLV10CarGas _gameinstanceref) (<= (Math|Random|RandomFloatinRange 0.0 1e+02) 25.0))
    (Default|ExtraGas _gameinstanceref))
  (Utilities|FlowControl|DelayUntilNextTick)
  (Audio|PlaySound2D "/Game/SFX/SC_Zombie_Death_Random.SC_Zombie_Death_Random" 1.0 1.0 0.0 0 0)
  (Actor|DestroyActor))

(event EventTick
  (params (DeltaSeconds :type Float%20%28single-precision%29))
  (bind _skeletalmesh (Variables|Default|GetSkeletalMesh))
  (bind _returnvalue (Transformation|GetWorldLocation _skeletalmesh))
  (|CallParentFunction DeltaSeconds)
  (Variables|Default|SetInterpSpeed (/ (Math|Vector|VectorLength (- _returnvalue (Variables|Default|GetPreviousLocation))) DeltaSeconds))
  (Variables|Default|SetPreviousLocation _returnvalue))

(fn ConstructionScript
  (|CallParentFunction))
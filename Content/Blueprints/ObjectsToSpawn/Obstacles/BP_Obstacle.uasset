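; BP_Obstacle is an obstacle that damages a car the first time something overlaps its HitBox.
; After a one-tick delay, it calls TakeDamage on the overlapping actor's AC_CarHealth component and plays a damage sound.
; An optional camera shake stops after half a second.
; The DoOnce is never reset here, so even an actor without health uses up the single trigger.
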(event OnComponentBeginOverlap(HitBox)
  (params (OverlappedComponent :type Primitive%20Component%20Object%20Reference) (OtherActor :type Actor%20Object%20Reference) (OtherComp :type Primitive%20Component%20Object%20Reference) (OtherBodyIndex :type Integer) (bFromSweep :type Boolean) (SweepResult :type Hit%20Result%20Structure%20%28by%20ref%29))
  (bind _returnvalue (Actor|GetComponentbyClass OtherActor "/Game/Blueprints/AC_CarHealth.AC_CarHealth_C"))
  (Utilities|FlowControl|DoOnce false
    (:Completed
      (Utilities|FlowControl|DelayUntilNextTick)
      (Utilities|IsValid _returnvalue
        (:Is%20Valid
          (Default|TakeDamage _returnvalue (Variables|Default|GetDamage))
          (Audio|PlaySound2D "/Game/SFX/Car_Sounds/Car_Damage_V2.Car_Damage_V2" 1.0 1.0 0.0 0 0)
          (Development|PrintString "Damage Taken")
          (if (Variables|Default|GetShouldTriggerShake)
            (Class|LegacyCameraShake|StartLegacyCameraShake (Game|GetPlayerCameraManager 0) "/Game/Blueprints/CS_ObstacleHit.CS_ObstacleHit_C" 0.6 "CameraLocal" "0, 0, 0")
            (Utilities|FlowControl|Delay 0.5)
            (CallFunction|StopCameraShake)))
        (:Is%20Not%20Valid
          (Development|PrintString "HealthRef Invalid" true true "(R=0.395833,G=0.000000,B=0.039531,A=1.000000)"))))))

(event Custom|StopCameraShake
  (Class|PlayerCameraManager|StopAllInstancesOfCameraShake (Game|GetPlayerCameraManager 0) "/Game/Blueprints/CS_ObstacleHit.CS_ObstacleHit_C" true)
  (Development|PrintString "Camera Shake Stop"))

(event EventBeginPlay
  (bind _asbp_game_instance (Utilities|Casting|CastToBP_GameInstance (Game|GetGameInstance)))
  (Variables|Default|SetGameInstanceRef _asbp_game_instance))

(fn ConstructionScript)
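; BP_ZenoFollower is an actor that trails the player's BP_Survivor pawn and carries a zombie spawner with it.
; On BeginPlay it targets the survivor, then spawns a BP_ZombieSpawner and attaches it to itself.
; Each Tick, when the target is at least FollowDis away, it moves toward it at constant MoveSpeed, keeping its height and yawing to face it.
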(event EventTick
  (params (DeltaSeconds :type Float%20%28single-precision%29))
  (bind _returnvalue (Transformation|GetActorLocation))
  (bind _movespeed (Variables|Default|GetMoveSpeed))
  (bind _target (Variables|Default|GetTarget))
  (bind _returnvalue_2 (Transformation|GetActorLocation _target))
  (bind _returnvalue_3 (Math|Interpolation|VInterptoConstant _returnvalue _returnvalue_2 DeltaSeconds _movespeed))
  (bind (_x _y) (Math|Vector|BreakVector _returnvalue_3))
  (Utilities|IsValid _target
    (:Is%20Valid
      (if (>= (Math|Vector|Distance(Vector) _returnvalue _returnvalue_2) (Variables|Default|GetFollowDis))
        (Transformation|SetActorLocationAndRotation (Math|Vector|MakeVector _x _y (.z (Transformation|GetActorLocation))) (Math|Rotator|MakeRotator 0.0 0.0 (.yaw (Math|Rotator|FindLookatRotation _returnvalue_3 _returnvalue_2))))))
    (:Is%20Not%20Valid
      (Development|PrintString "No Target Set"))))

(event EventBeginPlay
  (bind _asbp_survivor (Utilities|Casting|CastToBP_Survivor (Game|Player|GetPlayerPawn 0)))
  (Variables|Default|SetTarget _asbp_survivor)
  (bind _returnvalue (Game|SpawnActorfromClass "/Game/Blueprints/Zombies/BP_ZombieSpawner.BP_ZombieSpawner_C" (Transformation|GetActorTransform) "Undefined" "MultiplyWithRoot" 0 0))
  (Transformation|AttachActorToActor _returnvalue self "None" "KeepRelative" "KeepRelative" "KeepRelative" true))

(fn ConstructionScript)
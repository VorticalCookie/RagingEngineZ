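; BP_Grenade is a grenade actor that damages zombies in an area.
; It explodes 1.5 seconds after BeginPlay, or when its collision overlaps an actor with an AC_ZombieHealth component.
; The explosion runs a debug-drawn multi-sphere object trace at ExplosionRadius and calls TakeDamage on each hit actor's AC_ZombieHealth.
; DestroyActor sits inside the hit loop, so a blast with no hits leaves the grenade alive.
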(event OnComponentBeginOverlap(Collision)
  (params (OverlappedComponent :type Primitive%20Component%20Object%20Reference) (OtherActor :type Actor%20Object%20Reference) (OtherComp :type Primitive%20Component%20Object%20Reference) (OtherBodyIndex :type Integer) (bFromSweep :type Boolean) (SweepResult :type Hit%20Result%20Structure%20%28by%20ref%29))
  (Utilities|IsValid (Actor|GetComponentbyClass OtherActor "/Game/Blueprints/AC_ZombieHealth.AC_ZombieHealth_C")
    (:Is%20Valid
      (CallFunction|Explodes))))

(event Custom|Explodes
  (bind _explosionradius (Variables|Default|GetExplosionRadius))
  (bind _returnvalue (Transformation|GetWorldLocation _explosionradius))
  (bind (_outhits _returnvalue_2) (Collision|MultiSphereTraceForObjects _returnvalue _returnvalue 3e+02 (Variables|Default|GetObject%20Types) false 0 "ForDuration"))
  (if _returnvalue_2
    (bind _array_element (Utilities|Array|ForEachLoopwithBreak _outhits)
      (:LoopBody
        (Default|TakeDamage (Actor|GetComponentbyClass (.HitActor (Collision|BreakHitResult _array_element)) "/Game/Blueprints/AC_ZombieHealth.AC_ZombieHealth_C") (Variables|Default|GetDamage))
        (Actor|DestroyActor)))))

(event EventBeginPlay
  (Utilities|FlowControl|Delay 1.5)
  (CallFunction|Explodes))

(fn ConstructionScript)
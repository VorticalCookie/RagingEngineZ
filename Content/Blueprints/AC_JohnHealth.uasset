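; Health component for the player character John that applies incoming damage and reports death.
; TakeDamage ignores hits while BP_GameInstance reports gameplay blocked or IsInvincible is set, otherwise subtracts health and plays a hurt sound.
; It then calls the Death dispatcher at zero health or below, or CheckInvinsible if John survives.
; The node setting IsInvincible true is disconnected, so this component never enables invincibility itself.
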(event EventBeginPlay)

(event EventTick
  (params (DeltaSeconds :type Float%20%28single-precision%29)))

(fn TakeDamage
  (params (Damage :type Integer))
  (bind _asbp_game_instance (Utilities|Casting|CastToBP_GameInstance (Game|GetGameInstance)))
  (bind _isblocked (Default|IsGameplayBlocked _asbp_game_instance))
  (if (not _isblocked)
    (if (Variables|Default|GetIsInvincible?)
      (Development|PrintString "Player Invincible")
      (else
        (bind _output_get (Variables|Default|SetHealth (- (Variables|Default|GetHealth) Damage)))
        (Audio|PlaySound2D "/Game/SFX/John_hurt.John_hurt" 2.0 1.0 0.0 0 0)
        (if (<= _output_get 0)
          (Default|CallDeath)
          (else
            (Default|CallCheckInvinsible)))))))
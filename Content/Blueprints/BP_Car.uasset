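; Player car for the driving mode, switching between three lanes by swipe or A/D through a timeline scaled by the handling rate.
; BeginPlay initializes or restores gas and HP from BP_GameInstance, revives a dead car and adds the health UI and input context.
; Gas drains by subtracting elapsed game time; death or an empty tank hands off to on-foot play.
; The hurt box triggers BPI_Pickupable pickups.
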(event OnComponentBeginOverlap(HurtBox)
  (params (OverlappedComponent :type Primitive%20Component%20Object%20Reference) (OtherActor :type Actor%20Object%20Reference) (OtherComp :type Primitive%20Component%20Object%20Reference) (OtherBodyIndex :type Integer) (bFromSweep :type Boolean) (SweepResult :type Hit%20Result%20Structure%20%28by%20ref%29))
  ;[0.15 0.15 0.15 0.5] PowerUp
  (if (Utilities|DoesObjectImplementInterface OtherActor "/Game/Blueprints/DataStructures/BPI_Pickupable.BPI_Pickupable_C")
    (Class|BPIPickupable|OnPickedUp(Message) OtherActor self)
    (Development|PrintString "PowerUp!")))

(event Death(AC_CarHealth)
  (bind _returnvalue (Game|GetGameInstance))
  ;[0.15 0.15 0.15 0.5] On Death Switch to on Foot
  (Utilities|IsValid _returnvalue
    (:Is%20Valid
      (bind _asbp_game_instance (Utilities|Casting|CastToBP_GameInstance _returnvalue))
      (bind _output_get (Variables|Default|SetGame%20Instance _asbp_game_instance))
      (bind _isblocked (Default|IsGameplayBlocked _output_get))
      (if (not _isblocked)
        (Development|PrintString "Changing Scenes")
        (Variables|/Game/Blueprints/GameMode/BP_GameInstance.BP_GameInstance_C|SetCarCurrentGas (Variables|Default|GetGame%20Instance) (Variables|Default|GetTick%20Gas))
        (Variables|/Game/Blueprints/GameMode/BP_GameInstance.BP_GameInstance_C|SetCarMaxGas (Variables|Default|GetGame%20Instance) (Variables|Default|GetMaximum%20Gas))
        (Default|PlayTransition/Level (Variables|Default|GetGame%20Instance) "NewEnumerator0")))))

(event Custom|SideMovement
  (params (Axis :type Float%20%28double-precision%29))
  (bind _defaultsceneroot (Variables|Default|GetDefaultSceneRoot))
  (bind _returnvalue (Transformation|GetWorldLocation _defaultsceneroot))
  ;[0.15 0.15 0.15 0.5] Side Movement
  (Variables|Default|SetSide%20Movement true)
  (bind _finalspeed (Default|GetFinalHandlingRate (Variables|Default|GetGame%20Instance)))
  (Development|PrintString (Utilities|String|ToString(Float) _finalspeed))
  (Components|Timeline|SetPlayRate (Variables|Default|GetMovement) _finalspeed)
  (bind _side_movement (Timeline|Movement PlayFromStart)
    (:Update
      (Transformation|SetWorldLocation _defaultsceneroot (Math|Vector|MakeVector (.x _returnvalue) (* (+ (.y _side_movement) (Utilities|Select :Index (Variables|Default|GetCurrent%20Lane) :Option%200 -1.8e+02 :Option%201 0.0 :Option%202 -1.8e+02)) Axis) (.z _returnvalue)) false false))
    (:Finished
      (Variables|Default|SetCurrent%20Lane (+ (Variables|Default|GetCurrent%20Lane) (select (< Axis 0.0) -1 1)))
      (Variables|Default|SetSide%20Movement false))))

(event Custom|SwitchPowerUpType
  (params (NewPowerUpType :type CarPowerUpTypes%20Enum :default "NewEnumerator0"))
  ;[0.15 0.15 0.15 0.5] PowerUp
  (switch Utilities|FlowControl|Switch|SwitchonCarPowerUpTypes NewPowerUpType
    (:NewEnumerator0
      (Development|PrintString "PowerUpActivated"))))

(event Custom|Car_Gas
  (bind _game_instance (Variables|Default|GetGame%20Instance))
  (bind _ac_carhealth (Variables|Default|GetAC_CarHealth))
  ;[0.15 0.15 0.15 0.5] Out of Gas Switch to on Foot
  (bind _isblocked (Default|IsGameplayBlocked (Variables|Default|GetGame%20Instance)))
  (if (not _isblocked)
    (bind _output_get (Variables|Default|SetCurrent%20Gas (Variables|Default|GetCurrent%20Gas)))
    (bind _output_get_2 (Variables|Default|SetTick%20Gas (- _output_get (Utilities|Time|GetGameTimeinSeconds))))
    (Development|PrintString (Utilities|String|ToString(Float) _output_get_2) true true "(R=1.000000,G=0.954562,B=0.001897,A=1.000000)" 0.0 (Utilities|Name|MakeLiteralName "Gas Display"))
    (if (<= (- _output_get (Utilities|Time|GetGameTimeinSeconds)) 0.0)
      (Variables|/Game/Blueprints/GameMode/BP_GameInstance.BP_GameInstance_C|SetCarHP _game_instance (Variables|/Game/Blueprints/AC_CarHealth.AC_CarHealth_C|GetHealth _ac_carhealth))
      (Variables|/Game/Blueprints/GameMode/BP_GameInstance.BP_GameInstance_C|SetCarHP%20Max _game_instance (Variables|/Game/Blueprints/AC_CarHealth.AC_CarHealth_C|GetMax%20Car%20Health _ac_carhealth))
      (Default|OnFootOutOfGas _game_instance))))

(event Custom|AddGas
  (Variables|Default|SetCurrent%20Gas (+ (Variables|Default|GetCurrent%20Gas) 1e+01)))

(event Custom|Repair%20Gas
  (Variables|Default|SetCurrent%20Gas (+ (Variables|Default|GetCurrent%20Gas) (* (Variables|Default|GetMaximum%20Gas) 0.1))))

(event EventBeginPlay
  (bind _ac_carhealth (Variables|Default|GetAC_CarHealth))
  ;[0.15 0.15 0.15 0.5 50] Make Car gas consistent between game modes
  (bind _asbp_game_instance (Utilities|Casting|CastToBP_GameInstance (Game|GetGameInstance)))
  (Variables|Default|SetGame%20Instance _asbp_game_instance)
  (if (Variables|/Game/Blueprints/GameMode/BP_GameInstance.BP_GameInstance_C|GetCarGasInitialized (Variables|Default|GetGame%20Instance))
    (Variables|Default|SetMaximum%20Gas (Variables|/Game/Blueprints/GameMode/BP_GameInstance.BP_GameInstance_C|GetCarMaxGas (Variables|Default|GetGame%20Instance)))
    (Variables|Default|SetCurrent%20Gas (Variables|/Game/Blueprints/GameMode/BP_GameInstance.BP_GameInstance_C|GetCarCurrentGas (Variables|Default|GetGame%20Instance)))
    (else
      (bind _maxgas (Default|GetCarMaxGas (Variables|Default|GetGame%20Instance)))
      (bind _output_get (Variables|/Game/Blueprints/GameMode/BP_GameInstance.BP_GameInstance_C|SetCarMaxGas (Variables|Default|GetGame%20Instance) _maxgas))
      (Variables|/Game/Blueprints/GameMode/BP_GameInstance.BP_GameInstance_C|SetCarCurrentGas (Variables|Default|GetGame%20Instance) _output_get)
      (Variables|Default|SetMaximum%20Gas (Variables|/Game/Blueprints/GameMode/BP_GameInstance.BP_GameInstance_C|GetCarMaxGas (Variables|Default|GetGame%20Instance)))
      (Variables|Default|SetCurrent%20Gas (Variables|/Game/Blueprints/GameMode/BP_GameInstance.BP_GameInstance_C|GetCarCurrentGas (Variables|Default|GetGame%20Instance)))
      (Variables|/Game/Blueprints/GameMode/BP_GameInstance.BP_GameInstance_C|SetCarGasInitialized (Variables|Default|GetGame%20Instance) true)))
  ;[0.15 0.15 0.15 0.5 50] Make Car HP consistent between game modes
  (if (Variables|/Game/Blueprints/GameMode/BP_GameInstance.BP_GameInstance_C|GetCarHP_Initialized (Variables|Default|GetGame%20Instance))
    ;;[0.15 0.15 0.15 0.5] If car has died while driving, revive back with percentage of max hp
    (if (<= (Variables|/Game/Blueprints/GameMode/BP_GameInstance.BP_GameInstance_C|GetCarHP (Variables|Default|GetGame%20Instance)) 0)
      (Default|CarRevive (Variables|Default|GetGame%20Instance)))
    (else
      (bind _maxarmor (Default|GetCarMaxHealth (Variables|Default|GetGame%20Instance)))
      (Variables|/Game/Blueprints/GameMode/BP_GameInstance.BP_GameInstance_C|SetCarHP%20Max (Variables|Default|GetGame%20Instance) (Math|Float|Truncate _maxarmor))
      (Variables|/Game/Blueprints/GameMode/BP_GameInstance.BP_GameInstance_C|SetCarHP (Variables|Default|GetGame%20Instance) (Math|Float|Truncate _maxarmor))
      (Variables|/Game/Blueprints/GameMode/BP_GameInstance.BP_GameInstance_C|SetCarHP_Initialized (Variables|Default|GetGame%20Instance) true)))
  (Variables|/Game/Blueprints/AC_CarHealth.AC_CarHealth_C|SetMax%20Car%20Health _ac_carhealth (Variables|/Game/Blueprints/GameMode/BP_GameInstance.BP_GameInstance_C|GetCarHP%20Max (Variables|Default|GetGame%20Instance)))
  (Variables|/Game/Blueprints/AC_CarHealth.AC_CarHealth_C|SetHealth _ac_carhealth (Variables|/Game/Blueprints/GameMode/BP_GameInstance.BP_GameInstance_C|GetCarHP (Variables|Default|GetGame%20Instance)))
  (bind _returnvalue (UserInterface|CreateWidget "/Game/UI/UI_Car_Health.UI_Car_Health_C"))
  (UserInterface|Viewport|AddtoViewport _returnvalue 0)
  (bind _asbp_car_controller (Utilities|Casting|CastToBP_CarController (Game|GetPlayerController 0)))
  (Utilities|IsValid (PlayerController|LocalPlayerSubsystems|GetEnhancedInputLocalPlayerSubsystem _asbp_car_controller)
    (:Is%20Valid
      (Input|AddMappingContext (PlayerController|LocalPlayerSubsystems|GetEnhancedInputLocalPlayerSubsystem _asbp_car_controller) "/Game/Inputs/IMC_CarMovement.IMC_CarMovement" 0 "(bIgnoreAllPressedKeysUntilRelease=True,bForceImmediately=False,bNotifyUserSettings=False)"))))

(event EventTick
  (params (DeltaSeconds :type Float%20%28single-precision%29))
  ;[0.15 0.15 0.15 0.5] Out of Gas Switch to on Foot
  (CallFunction|CarGas))

(event Input|KeyboardEvents|A
  (params (Key :type Key%20Structure :default "None"))
  ;[0.15 0.15 0.15 0.5] Set Ups Touch Controller
  (:Pressed
    (if (and (> (Variables|Default|GetCurrent%20Lane) 0) (not (Variables|Default|GetSide%20Movement)))
      (CallFunction|SideMovement -1.0))))

(event Input|KeyboardEvents|D
  (params (Key :type Key%20Structure :default "None"))
  ;[0.15 0.15 0.15 0.5] Set Ups Touch Controller
  (:Pressed
    (if (and (< (Variables|Default|GetCurrent%20Lane) 2) (not (Variables|Default|GetSide%20Movement)))
      (CallFunction|SideMovement 1.0))))

(event Input|TouchEvents|InputTouch
  (params (Location :type Vector) (FingerIndex :type ETouchIndex%20Enum))
  (bind _returnvalue (Math|Vector2D|MakeVector2D (.x Location) (.y Location)))
  ;[0.15 0.15 0.15 0.5] Set Ups Touch Controller
  (:Pressed
    (Variables|Default|SetTouch%20Start%20Location _returnvalue)
    (Variables|Default|SetTouch%20Active true))
  (:Released
    (Variables|Default|SetTouch%20Active false))
  (:Moved
    (Variables|Default|SetCurrent%20Touch%20Location _returnvalue)
    (if (Variables|Default|GetTouch%20Active)
      (Utilities|FlowControl|Sequence
        (:then_0
          (if (> (.X (Math|Vector2D|BreakVector2D (- (Variables|Default|GetCurrent%20Touch%20Location) (Variables|Default|GetTouch%20Start%20Location)))) (Variables|Default|GetSwipe%20Threshold))
            (if (and (< (Variables|Default|GetCurrent%20Lane) 2) (not (Variables|Default|GetSide%20Movement)))
              (CallFunction|SideMovement 1.0))))
        (:then_1
          (if (< (.X (Math|Vector2D|BreakVector2D (- (Variables|Default|GetCurrent%20Touch%20Location) (Variables|Default|GetTouch%20Start%20Location)))) (* (Variables|Default|GetSwipe%20Threshold) -1.0))
            (if (and (> (Variables|Default|GetCurrent%20Lane) 0) (not (Variables|Default|GetSide%20Movement)))
              (CallFunction|SideMovement -1.0))))))))

(fn ConstructionScript)
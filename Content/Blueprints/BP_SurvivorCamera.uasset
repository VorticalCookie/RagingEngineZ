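; Survivor camera actor that trails the player's BP_Survivor pawn.
; On BeginPlay it targets that pawn and derives its move speed from the character's max walk speed, less a fixed offset.
; Each tick, once the 3D distance reaches FollowDis, it steps toward the target's X and Y with constant-speed interpolation, printing a message if no valid target exists.
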(event EventBeginPlay
  (bind _asbp_survivor (Utilities|Casting|CastToBP_Survivor (Game|Player|GetPlayerPawn 0)))
  (bind _output_get (Variables|Default|SetTarget _asbp_survivor))
  (Variables|Default|SetMoveSpeed (- (Variables|/Script/Engine.CharacterMovementComponent|GetMaxWalkSpeed (Variables|/Script/Engine.Character|GetCharacterMovement _output_get)) 5e+02)))

(event EventTick
  (params (DeltaSeconds :type Float%20%28single-precision%29))
  (bind _returnvalue (Transformation|GetActorLocation))
  (bind _target (Variables|Default|GetTarget))
  (bind _movespeed (Variables|Default|GetMoveSpeed))
  (bind _returnvalue_2 (Transformation|GetActorLocation _target))
  (bind _returnvalue_3 (Math|Interpolation|VInterptoConstant _returnvalue _returnvalue_2 DeltaSeconds _movespeed))
  (bind (_x _y) (Math|Vector|BreakVector _returnvalue_3))
  (Utilities|IsValid _target
    (:Is%20Valid
      (if (>= (Math|Vector|Distance(Vector) _returnvalue _returnvalue_2) (Variables|Default|GetFollowDis))
        (Transformation|SetActorLocation (Math|Vector|MakeVector _x _y 0.0) false false)))
    (:Is%20Not%20Valid
      (Development|PrintString "No Target Set"))))

(fn ConstructionScript)
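; BP_Turret is an auto-firing turret that removes itself at BeginPlay unless the game instance's LV10CarArmor flag is set.
; A delay loop paced by ShotDelay repeatedly plays a shotgun sound and spawns a fixed-damage BP_Projectile, whether or not zombies are present.
; Each Tick it finds the nearest BP_Zombie and snaps its yaw toward it without interpolation, or to zero when none exist.
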(event EventBeginPlay
  (Utilities|FlowControl|Sequence
    (:then_0
      (bind _asbp_game_instance (Utilities|Casting|CastToBP_GameInstance (Game|GetGameInstance)))
      (if (not (Variables|/Game/Blueprints/GameMode/BP_GameInstance.BP_GameInstance_C|GetLV10CarArmor _asbp_game_instance))
        (Actor|DestroyActor)))
    (:then_1
      (Utilities|DelayLoop (Variables|Default|GetShotDelay) true
        (:Loop%20Body
          (Utilities|FlowControl|Delay (Variables|Default|GetShotDelay))
          (Audio|PlaySound2D "/Game/Audio/Shotgun_Shoot_8Bit.Shotgun_Shoot_8Bit" 1.0 1.0 0.0 0 0)
          (Game|SpawnActorfromClass "/Game/Blueprints/Projectiles/BP_Projectile.BP_Projectile_C" (Utilities|SpawnTransform) "Undefined" "MultiplyWithRoot" 0 10 false 0))))))

(event EventTick
  (params (DeltaSeconds :type Float%20%28single-precision%29))
  (bind _returnvalue (Transformation|GetActorLocation))
  (bind _outactors (Actor|GetAllActorsOfClass "/Game/Blueprints/Zombies/BP_Zombie.BP_Zombie_C"))
  (if (not (== (Utilities|Array|Length _outactors) 0))
    (Variables|Default|SetTargetRotation (.yaw (Math|Rotator|FindLookatRotation _returnvalue (Transformation|GetActorLocation (.ReturnValue (Actor|FindNearestActor _returnvalue _outactors))))))
    (else
      (Variables|Default|SetTargetRotation 0.0)))
  (CallFunction|SnapPlayer))

(fn ConstructionScript)

(fn SnapPlayer
  (bind _returnvalue (Transformation|GetActorRotation))
  (Transformation|SetActorRotation (Math|Rotator|MakeRotator (.roll _returnvalue) (.pitch _returnvalue) (Variables|Default|GetTargetRotation)))
  (return))
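; BP_Projectile is a projectile actor that damages zombies.
; When its Sphere overlaps an actor with an AC_ZombieHealth component, it passes Damage to that component's TakeDamage and destroys itself.
; It also destroys itself when ProjectileMovement stops.
; Unconnected leftover nodes that would set velocity from the look-at yaw toward the nearest BP_Zombie never run, so the graph does no homing.
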(event OnProjectileStop(ProjectileMovement)
  (params (ImpactResult :type Hit%20Result%20Structure%20%28by%20ref%29))
  (Actor|DestroyActor))

(event OnComponentBeginOverlap(Sphere)
  (params (OverlappedComponent :type Primitive%20Component%20Object%20Reference) (OtherActor :type Actor%20Object%20Reference) (OtherComp :type Primitive%20Component%20Object%20Reference) (OtherBodyIndex :type Integer) (bFromSweep :type Boolean) (SweepResult :type Hit%20Result%20Structure%20%28by%20ref%29))
  (bind _returnvalue (Actor|GetComponentbyClass OtherActor "/Game/Blueprints/AC_ZombieHealth.AC_ZombieHealth_C"))
  (Utilities|IsValid _returnvalue
    (:Is%20Valid
      (Default|TakeDamage _returnvalue (Variables|Default|GetDamage))
      (Actor|DestroyActor))))

(fn ConstructionScript)
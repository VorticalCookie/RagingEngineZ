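; Projectile that damages zombies on overlap and ricochets once toward another nearby target.
; The first hit runs a sphere trace that ignores the survivor, attempts to drop the nearest actor, then redirects velocity horizontally toward the nearest remaining one.
; A flag destroys the projectile on its next zombie hit.
; It also destroys itself when movement stops, or after a short delay if the trace finds nothing.
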(event OnProjectileStop(ProjectileMovement)
  (params (ImpactResult :type Hit%20Result%20Structure%20%28by%20ref%29))
  (Actor|DestroyActor))

(event OnComponentBeginOverlap(Sphere)
  (params (OverlappedComponent :type Primitive%20Component%20Object%20Reference) (OtherActor :type Actor%20Object%20Reference) (OtherComp :type Primitive%20Component%20Object%20Reference) (OtherBodyIndex :type Integer) (bFromSweep :type Boolean) (SweepResult :type Hit%20Result%20Structure%20%28by%20ref%29))
  (bind _returnvalue (Actor|GetComponentbyClass OtherActor "/Game/Blueprints/AC_ZombieHealth.AC_ZombieHealth_C"))
  (Utilities|IsValid _returnvalue
    (:Is%20Valid
      (Default|TakeDamage _returnvalue (Variables|Default|GetDamage) (Variables|Default|GetCanKnockback?))
      (if (Variables|Default|GetHasRicochet?)
        (Actor|DestroyActor)
        (else
          (CallFunction|Ricochet))))))

(event Custom|Ricochet
  (bind _returnvalue (Transformation|GetActorLocation))
  (bind _returnvalue_2 (Transformation|GetActorLocation))
  (bind _returnvalue_3 (Transformation|GetActorLocation))
  (bind (_x _y) (Math|Vector|BreakVector _returnvalue_3))
  (bind _returnvalue_4 (Actor|GetActorOfClass "/Game/Blueprints/BP_Survivor.BP_Survivor_C"))
  (bind (_outhits _returnvalue_5) (Collision|MultiSphereTraceForObjects _returnvalue _returnvalue 3e+02 (Variables|Default|GetObject%20Types) false (Utilities|Array|MakeArray _returnvalue_4) "None"))
  (if _returnvalue_5
    (for _array_element _outhits
      (Utilities|Array|RemoveItem (Utilities|Array|MakeArray (.HitActor (Collision|BreakHitResult _array_element)) 0) (.ReturnValue (Actor|FindNearestActor _returnvalue_2 (Utilities|Array|MakeArray (.HitActor (Collision|BreakHitResult _array_element)) 0)))))
    (Variables|Default|SetHasRicochet? true)
    (Variables|/Script/Engine.MovementComponent|SetVelocity (Variables|Default|GetProjectileMovement) (* (Math|Vector|Normalize (- (Math|Vector|MakeVector (.X (Math|Vector|BreakVector (Transformation|GetActorLocation (.ReturnValue (Actor|FindNearestActor _returnvalue_2 (Utilities|Array|MakeArray (.HitActor (Collision|BreakHitResult _array_element)) 0)))))) (.Y (Math|Vector|BreakVector (Transformation|GetActorLocation (.ReturnValue (Actor|FindNearestActor _returnvalue_2 (Utilities|Array|MakeArray (.HitActor (Collision|BreakHitResult _array_element)) 0)))))) 0.0) (Math|Vector|MakeVector _x _y 0.0))) 1e+03))
    (else
      (Variables|Default|SetHasRicochet? true)
      (Development|PrintString "No enemies nearby")
      (Utilities|FlowControl|Delay 2.0)
      (Actor|DestroyActor))))

(fn ConstructionScript)
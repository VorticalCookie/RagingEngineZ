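; BP_SurvivorGameMode is the game mode that tracks the live zombie count and caps spawning in the survivor game.
; Increase and decrease events maintain the count, with each decrease also recording a kill on BP_GameInstance.
; ShouldZombiesSpawn returns true while the count is at or below MaxZombieCap.
; On BeginPlay it has the GameInstance add the main HUD and, if transitioning, creates a UI_Transition widget to end the transition.
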(event Custom|Decrease%20Zombie%20Count
  ;[0.15 0.15 0.15 0.5] Manage ZombieCount
  (Math|Integer|DecrementInt (Variables|Default|GetCurrent%20Zombie%20Count)
    (:%20%20
      (Default|AddZombieKills (Variables|Default|GetGame%20Instance)))))

(event Custom|Increase%20Zombie%20Count
  ;[0.15 0.15 0.15 0.5] Manage ZombieCount
  (Math|Integer|IncrementInt (Variables|Default|GetCurrent%20Zombie%20Count)))

(event EventBeginPlay
  (Utilities|FlowControl|Sequence
    (:then_0
      (bind _asbp_game_instance (Utilities|Casting|CastToBP_GameInstance (Game|GetGameInstance)))
      (bind _output_get (Variables|Default|SetGame%20Instance _asbp_game_instance))
      (Utilities|IsValid _output_get
        (:Is%20Valid
          (Default|AddMainHUD _output_get))))
    (:then_1
      (if (Variables|/Game/Blueprints/GameMode/BP_GameInstance.BP_GameInstance_C|GetIsTransitioning (Variables|Default|GetGame%20Instance))
        (bind _returnvalue (UserInterface|CreateWidget "/Game/UI/UI_Transition.UI_Transition_C" (Game|GetPlayerController 0)))
        (UserInterface|Viewport|AddtoViewport _returnvalue 0)
        (Default|EndTransition _returnvalue)))))

(fn ConstructionScript)

(fn ShouldZombiesSpawn
  ;[0.15 0.15 0.15 0.5] If Zombies reach the cap no more zombies will spawn
  (return (<= (Variables|Default|GetCurrent%20Zombie%20Count) (Variables|Default|GetMax%20Zombie%20Cap))))
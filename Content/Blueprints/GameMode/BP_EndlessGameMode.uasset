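; Game mode for an endless three-lane runner that builds the track from BP_FloorTile actors.
; BeginPlay chains an initial run of tiles from a placed tile's AttachPoint; AddNewTile appends another after the last active tile.
; Each tile gets a random lane pattern, shuffled across lanes, that places random obstacles or power-ups, plus random scenery on both sides.
; IncreaseSpeed is an empty stub.
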(event Custom|SpawnLaneObjects
  (params (Random%20Pattern%20Index :type Integer))
  (bind _objectsspawnpattern (Variables|Default|GetObjectsSpawnPattern))
  (bind _output (Utilities|Array|Get(acopy) _objectsspawnpattern Random%20Pattern%20Index))
  (bind (_lanel _lanem _laner) (Utilities|Struct|BreakStructure_LaneSpawn _output))
  ;[0.15 0.15 0.15 0.5] SpawnObjects
  ;;[0.15 0.15 0.15 0.5] Adds Randomness
  (bind _output_get (Variables|Default|SetLaneObjects (Utilities|Array|MakeArray _lanel _lanem _laner)))
  (Utilities|Array|Shuffle _output_get)
  (for (_array_element _array_index) (Variables|Default|GetLaneObjects)
    (switch Utilities|FlowControl|Switch|SwitchonEnum_ObjectsToSpawn _array_element
      (:NewEnumerator0
        (Default|SpawnObstacle (Variables|Default|GetBP%20Floor%20Ref) (CallFunction|GetRandomObstacle) _array_index))
      (:NewEnumerator1
        (Default|SpawnPowerUp (Variables|Default|GetBP%20Floor%20Ref) (CallFunction|GetRandomPowerUp) _array_index)))))

(event Custom|InitialSpawn
  ;[0.15 0.15 0.15 0.5] TileSpawn
  (bind _returnvalue (Game|SpawnActorfromClass "/Game/Blueprints/BP_FloorTile.BP_FloorTile_C" (Math|Transform|MakeTransform (.location (Variables|Default|GetNewTilePos)) (.rotation (Variables|Default|GetNewTilePos)) "1.000000,1.000000,1.000000") "Undefined" "MultiplyWithRoot" 0 0))
  (Variables|Default|SetBP%20Floor%20Ref _returnvalue)
  (Utilities|Array|Add (Variables|Default|GetActiveTiles) _returnvalue)
  (Variables|Default|SetNewTilePos (Transformation|GetWorldTransform (Variables|/Game/Blueprints/BP_FloorTile.BP_FloorTile_C|GetAttachPoint _returnvalue)))
  (CallFunction|SpawnLaneObjects (Math|Random|RandomIntegerinRange 0 (- (Utilities|Array|Length (Variables|Default|GetObjectsSpawnPattern)) 1)))
  (Default|SpawnEnvironment (Variables|Default|GetBP%20Floor%20Ref) (CallFunction|GetRandomEnvironment) (CallFunction|GetRandomEnvironment)))

(event Custom|Increase%20Speed)

(event EventBeginPlay
  ;[0.15 0.15 0.15 0.5] Spawn Initial Tiles
  (bind _returnvalue (Actor|GetActorOfClass "/Game/Blueprints/BP_FloorTile.BP_FloorTile_C"))
  (Variables|Default|SetNewTilePos (Transformation|GetWorldTransform (Variables|/Game/Blueprints/BP_FloorTile.BP_FloorTile_C|GetAttachPoint _returnvalue)))
  (for _index (range 0 5)
    (CallFunction|InitialSpawn)))

(event EventAddNewTile
  (bind _activetiles (Variables|Default|GetActiveTiles))
  ;[0.15 0.15 0.15 0.5] TileSpawn
  (bind _output_get (Variables|Default|SetNewTilePos (Transformation|GetWorldTransform (Variables|/Game/Blueprints/BP_FloorTile.BP_FloorTile_C|GetAttachPoint (Utilities|Array|Get(acopy) _activetiles (Utilities|Array|LastIndex _activetiles))))))
  (bind _returnvalue (Game|SpawnActorfromClass "/Game/Blueprints/BP_FloorTile.BP_FloorTile_C" (Math|Transform|MakeTransform (.location _output_get) (.rotation _output_get) "1.000000,1.000000,1.000000") "Undefined" "MultiplyWithRoot" 0 0))
  (bind _output_get_2 (Variables|Default|SetBP%20Floor%20Ref _returnvalue))
  (Utilities|Array|Add (Variables|Default|GetActiveTiles) _returnvalue)
  (CallFunction|SpawnLaneObjects (Math|Random|RandomIntegerinRange 0 (- (Utilities|Array|Length (Variables|Default|GetObjectsSpawnPattern)) 1)))
  (Default|SpawnEnvironment (Variables|Default|GetBP%20Floor%20Ref) (CallFunction|GetRandomEnvironment) (CallFunction|GetRandomEnvironment)))

(fn ConstructionScript)

(fn GetRandomObstacle
  (bind _obstacleclasses (Variables|Default|GetObstacleClasses))
  (return (Utilities|Array|Get(acopy) _obstacleclasses (Math|Random|RandomIntegerinRange 0 (- (Utilities|Array|Length _obstacleclasses) 1)))))

(fn GetRandomPowerUp
  (bind _powerupclasses (Variables|Default|GetPowerUpClasses))
  (return (Utilities|Array|Get(acopy) _powerupclasses (Math|Random|RandomIntegerinRange 0 (- (Utilities|Array|Length _powerupclasses) 1)))))

(fn GetRandomEnvironment
  (bind _environmentclasses (Variables|Default|GetEnvironmentClasses))
  (return (Utilities|Array|Get(acopy) _environmentclasses (Math|Random|RandomIntegerinRange 0 (- (Utilities|Array|Length _environmentclasses) 1)))))
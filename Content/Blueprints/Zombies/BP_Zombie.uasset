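; Zombie enemy character that damages the survivor player and reports spawns and deaths to the survivor game mode's zombie count.
; On BeginPlay it takes bonus health and a luck-based drop chance from the game instance.
; An AI task triggers damage, while a separate event plays a gated attack montage.
; Health component events drive knockback, temporary stun, and death, which awards money and may drop repair parts, ammo or gas.
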(event Death(AC_ZombieHealth)
  ;[0.15 0.15 0.15 0.5] Decrease Zombie Count
  (bind _asbp_survivor_game_mode (Utilities|Casting|CastToBP_SurvivorGameMode (Game|GetGameMode)))
  (Default|AddMoney (Variables|Default|GetGame%20Instance))
  (Default|DecreaseZombieCount _asbp_survivor_game_mode)
  (Utilities|FlowControl|DelayUntilNextTick)
  (CallFunction|DropResource)
  (Audio|PlaySound2D "/Game/SFX/Zombie_Sounds/SC_Zombie_Death_Random.SC_Zombie_Death_Random" 1.0 1.0 0.0 0 0)
  (Actor|DestroyActor))

(event Knockback(AC_ZombieHealth)
  (bind _returnvalue (Transformation|GetActorLocation))
  (bind _returnvalue_2 (Game|GetPlayerCharacter 0))
  (bind _returnvalue_3 (Transformation|GetActorLocation _returnvalue_2))
  (bind _returnvalue_4 (- _returnvalue _returnvalue_3))
  (bind _returnvalue_5 (Math|Vector|Normalize _returnvalue_4))
  (bind _returnvalue_6 (* _returnvalue_5 1e+03))
  (Character|LaunchCharacter (Math|Vector|MakeVector (.x _returnvalue_6) (.y _returnvalue_6) 1.5e+02) true true))

(event Stun(AC_ZombieHealth)
  (bind _charactermovement (Variables|Character|GetCharacterMovement))
  (Development|PrintString "Stun")
  (Variables|/Script/Engine.CharacterMovementComponent|SetMaxWalkSpeed _charactermovement 0.0)
  (Utilities|FlowControl|Delay 3.0)
  (Variables|/Script/Engine.CharacterMovementComponent|SetMaxWalkSpeed _charactermovement 175.0))

(event Custom|Damage%20Player
  (bind _survivor_ref (Variables|Default|GetSurvivor_Ref))
  (bind _returnvalue (Actor|GetComponentbyClass _survivor_ref "/Game/Blueprints/AC_JohnHealth.AC_JohnHealth_C"))
  ;[0.15 0.15 0.15 0.5] Attack Player Logic, this is triggered in the Task on the Sequence
  (Utilities|FlowControl|DelayUntilNextTick)
  (Utilities|IsValid _returnvalue
    (:Is%20Valid
      (Default|TakeDamage _returnvalue (Variables|Default|GetZombieDamage))
      (Development|PrintString "Dealing Damage!"))))

(event Custom|Drop%20Resource
  ;[0.15 0.15 0.15 0.5] On Zombie kill, random chance to drop resource or no resource
  (if (<= (Math|Random|RandomIntegerinRange 1 100) (Variables|Default|GetDrop%20Chance))
    (Game|SpawnActorfromClass (Utilities|Select :Index (Math|Random|RandomInteger 3) :Option%200 "/Game/Blueprints/ObjectsToSpawn/PowerUps/BP_Repair_Parts.BP_Repair_Parts_C" :Option%201 "/Game/Blueprints/ObjectsToSpawn/PowerUps/BP_Ammo.BP_Ammo_C" :Option%202 "/Game/Blueprints/ObjectsToSpawn/PowerUps/BP_GasPickup.BP_GasPickup_C" :Option%203 0) (Math|Transform|MakeTransform (Transformation|GetWorldLocation (Variables|Character|GetMesh)) "-60.000000,0.000000,0.000000" "1.000000,1.000000,1.000000") "Undefined" "MultiplyWithRoot" 0 0)
    (else
      (Development|PrintString "No Powerup"))))

(event Custom|Attack%20Anim
  ;[0.15 0.15 0.15 0.5] Plays Attack Animation
  (if (not (Variables|Default|GetIsAttacking))
    (Variables|Default|SetIsAttacking true)
    (Animation|PlayAnimMontage "/Game/Models/Animations/Zombie/AM_ZombieAttack.AM_ZombieAttack" 1.0 "None")
    (Utilities|FlowControl|Delay 1.16)
    (Variables|Default|SetIsAttacking false)))

(event EventBeginPlay
  (bind _ac_zombiehealth (Variables|Default|GetAC_ZombieHealth))
  ;[0.15 0.15 0.15 0.5] Increase Zombie Count when spawned
  (Class|AudioMixerBlueprintLibrary|PrimeSoundCueforPlayback "/Game/SFX/Zombie_Sounds/SC_Zombie_Death_Random.SC_Zombie_Death_Random")
  (bind _asbp_survivor_game_mode (Utilities|Casting|CastToBP_SurvivorGameMode (Game|GetGameMode)))
  (Default|IncreaseZombieCount _asbp_survivor_game_mode)
  ;;[0.15 0.15 0.15 0.5] Could be optimize by putting this ref into game instance
  (bind _asbp_survivor (Utilities|Casting|CastToBP_Survivor (Game|Player|GetPlayerPawn 0)))
  (Variables|Default|SetSurvivor_Ref _asbp_survivor)
  (bind _asbp_game_instance (Utilities|Casting|CastToBP_GameInstance (Game|GetGameInstance)))
  (bind _output_get (Variables|Default|SetGame%20Instance _asbp_game_instance))
  (Variables|/Game/Blueprints/AC_ZombieHealth.AC_ZombieHealth_C|SetHealth _ac_zombiehealth (+ (Variables|/Game/Blueprints/AC_ZombieHealth.AC_ZombieHealth_C|GetHealth _ac_zombiehealth) (Variables|/Game/Blueprints/GameMode/BP_GameInstance.BP_GameInstance_C|GetZombieExtraHealth _output_get)))
  (bind _johnluck (Default|GetJohnLuck _output_get))
  (Variables|Default|SetDrop%20Chance _johnluck))

(fn ConstructionScript)
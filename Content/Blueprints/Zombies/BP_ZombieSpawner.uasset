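; BP_ZombieSpawner spawns staggered groups of zombies at random reachable nav mesh points within a radius around itself.
; It finds the RecastNavMesh, retrying until valid, and spawns at BeginPlay, then on a looping timer when the GameMode allows.
; SpawnZombies re-calls itself after short random delays, capped by a DoN reset each timer tick.
; The GameMode's SpawnLevel sets DifficultyLevel, widening the random pick toward tougher zombie classes.
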(event Custom|Find%20Nav%20Mesh
  ;[0.15 0.15 0.15 0.5] Nav mesh ref
  (bind _outactors (Actor|GetAllActorsOfClass "/Script/NavigationSystem.RecastNavMesh"))
  (Utilities|IsValid (Utilities|Array|Get(acopy) _outactors)
    (:Is%20Valid
      (Variables|Default|SetNav%20Data (Utilities|Array|Get(acopy) _outactors)))
    (:Is%20Not%20Valid
      (Utilities|FlowControl|Delay 0.2)
      (CallFunction|FindNavMesh))))

(event Custom|Spawn%20Zombies
  (bind _returnvalue (Transformation|GetActorLocation))
  (bind _spawn_radius (Variables|Default|GetSpawn%20Radius))
  (bind _nav_data (Variables|Default|GetNav%20Data))
  (bind (_randomlocation _returnvalue_2) (AI|Navigation|GetRandomReachablePointinRadius _returnvalue _spawn_radius _nav_data 0))
  ;[0.15 0.15 0.15 0.5] Spawn zombie logic in 3s
  (bind _counter (Utilities|FlowControl|DoN (Variables|Default|GetSpawn%20Group%20Size))
    (:Exit
      (if _returnvalue_2
        (Game|SpawnActorfromClass (CallFunction|GetRandomZombieIndex) (Math|Conversions|ToTransform(Vector) _randomlocation) "AdjustIfPossibleButAlwaysSpawn" "MultiplyWithRoot" 0 0)
        (if (< _counter (Variables|Default|GetSpawn%20Group%20Size))
          (Utilities|FlowControl|Delay (Math|Random|RandomFloatinRange 0.2 0.7))
          (CallFunction|SpawnZombies))))))

(event Custom|Reset%20Spawn%20Group
  (bind _returnvalue (Transformation|GetActorLocation))
  (bind _spawn_radius (Variables|Default|GetSpawn%20Radius))
  (bind _nav_data (Variables|Default|GetNav%20Data))
  (bind (_randomlocation _returnvalue_2) (AI|Navigation|GetRandomReachablePointinRadius _returnvalue _spawn_radius _nav_data 0))
  ;[0.15 0.15 0.15 0.5] Spawn zombie logic in 3s
  (Utilities|FlowControl|DoN (Variables|Default|GetSpawn%20Group%20Size)) ; enters at Reset
)

(event Custom|Spawn%20Timer%20Expired
  ;[0.15 0.15 0.15 0.5] Check if zombies can spawn
  (CallFunction|ResetSpawnGroup)
  (bind _asbp_survivor_game_mode (Utilities|Casting|CastToBP_SurvivorGameMode (Game|GetGameMode)))
  (if (Default|ShouldZombiesSpawn _asbp_survivor_game_mode)
    (CallFunction|SpawnZombies)
    (Variables|Default|SetDifficultyLevel (Variables|/Game/Blueprints/GameMode/BP_SurvivorGameMode.BP_SurvivorGameMode_C|GetSpawnLevel _asbp_survivor_game_mode))))

(event EventBeginPlay
  (Utilities|FlowControl|Sequence
    (:then_0
      (CallFunction|FindNavMesh))
    (:then_1
      (CallFunction|SpawnZombies))
    (:then_3
      (Utilities|Time|SetTimerbyEvent (delegate Custom|Spawn%20Timer%20Expired) (Variables|Default|GetSpawn%20Delay) true))))

(fn ConstructionScript)

(fn GetRandomZombieIndex
  (return (Utilities|Select :Index (Math|Random|RandomInteger (Math|Integer|Clamp(Integer) (Variables|Default|GetDifficultyLevel) 0 10)) :Option%200 "/Game/Blueprints/Zombies/BP_Zombie.BP_Zombie_C" :Option%201 "/Game/Blueprints/Zombies/BP_Zombie.BP_Zombie_C" :Option%202 "/Game/Blueprints/Zombies/BP_Zombie.BP_Zombie_C" :Option%203 "/Game/Blueprints/Zombies/BP_Zombie.BP_Zombie_C" :Option%204 "/Game/Blueprints/Zombies/BP_Zombie_Med.BP_Zombie_Med_C" :Option%205 "/Game/Blueprints/Zombies/BP_Zombie_Med.BP_Zombie_Med_C" :Option%206 "/Game/Blueprints/Zombies/BP_Zombie_Med.BP_Zombie_Med_C" :Option%207 "/Game/Blueprints/Zombies/BP_Zombie_Heavy.BP_Zombie_Heavy_C" :Option%208 "/Game/Blueprints/Zombies/BP_Zombie_Heavy.BP_Zombie_Heavy_C" :Option%209 "/Game/Blueprints/Zombies/BP_Zombie_Boss.BP_Zombie_Boss_C")))